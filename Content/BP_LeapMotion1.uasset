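; Leap Motion test pawn that visualizes tracked hands with debug spheres and reports hand gestures.
; BeginPlay adds a Leap controller, optimizes it for HMD, and enables gestures and camera images.
; Finger and arm joint positions are offset forward and down, rotated by control rotation, and drawn relative to the actor.
; Grab, pinch and swipe events print messages, while raw sensor images pass to MyHud as a texture.
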(event EventBeginPlay
  (Development|PrintString "begin")
  (bind _returnvalue (AddComponent|AddLeapController))
  (bind _output_get (Variables|Default|SetLeapController _returnvalue))
  (Class|LeapController|OptimizeforHMD _output_get false true true)
  (Class|LeapController|EnableGesture _output_get "GESTURE_TYPE_SWIPE" true)
  (Class|LeapController|EnableGesture _output_get "GESTURE_TYPE_CIRCLE" true)
  (Class|LeapController|EnableGesture _output_get "GESTURE_TYPE_SCREEN_TAP" true)
  (Class|LeapController|EnableGesture _output_get "GESTURE_TYPE_KEY_TAP" true)
  (Class|LeapController|EnableImageSupport _output_get true true false))

(event EventLeapFingerMoved
  (params (finger :type Leap%20Finger%20Object%20Reference))
  (CallFunction|DrawDebugSphereatActor (Variables|/Script/LeapMotion.LeapPointable|GetTipPosition finger) 1.0)
  (CallFunction|DrawDebugSphereatActor (Variables|/Script/LeapMotion.LeapBone|GetCenter (Variables|/Script/LeapMotion.LeapFinger|GetMetacarpal finger)) 1.0)
  (CallFunction|DrawDebugSphereatActor (Variables|/Script/LeapMotion.LeapBone|GetCenter (Variables|/Script/LeapMotion.LeapFinger|GetProximal finger)) 1.0)
  (CallFunction|DrawDebugSphereatActor (Variables|/Script/LeapMotion.LeapBone|GetCenter (Variables|/Script/LeapMotion.LeapFinger|GetIntermediate finger)) 1.0))

(event EventRawImageReceived
  (params (texture :type Texture%202D%20Object%20Reference) (image :type Leap%20Image%20Object%20Reference))
  (bind _asmy_hud (Utilities|Casting|CastToMyHud (HUD|GetHUD (Game|GetPlayerController 0))))
  (Variables|/Game/MyHud.MyHud_C|SetLeap%20Texture _asmy_hud texture))

(event EventLeapHandPinched
  (params (strength :type Float%20%28single-precision%29) (hand :type Leap%20Hand%20Object%20Reference))
  ;[1 1 1] Leap motion events handler
  (Development|PrintString "pinched" true true "(R=0.000000,G=1.000000,B=0.331943,A=1.000000)" 1.0))

(event EventLeapHandMoved
  (params (hand :type Leap%20Hand%20Object%20Reference))
  (bind _arm (Variables|/Script/LeapMotion.LeapHand|GetArm hand))
  (CallFunction|DrawDebugSphereatActor (Variables|/Script/LeapMotion.LeapArm|GetWristPosition _arm) 2.0)
  (CallFunction|DrawDebugSphereatActor (Variables|/Script/LeapMotion.LeapArm|GetElbowPosition _arm) 4.0))

(event EventLeapHandGrabbed
  (params (strength :type Float%20%28single-precision%29) (hand :type Leap%20Hand%20Object%20Reference))
  ;[1 1 1] Leap motion events handler
  (Development|PrintString "LeapHandGrabbed" true true "(R=1.000000,G=0.000000,B=0.808155,A=1.000000)" 1.0))

(event EventSwipeGestureDetected
  (params (gesture :type Leap%20Swipe%20Gesture%20Object%20Reference))
  ;[1 1 1] Leap motion events handler
  (Development|PrintString "Swipe" true true "(R=0.000000,G=0.660000,B=1.000000,A=1.000000)" 1.0))

(fn ConstructionScript)

(fn DrawDebugSphereatActor
  (params (Location :type Vector) (Radius :type Float%20%28single-precision%29))
  (Rendering|Debug|DrawDebugSphere (+ (Math|Vector|RotateVector (+ Location "75.000000, 0,-20.000000") (Pawn|GetControlRotation :!class /Script/Engine.Pawn)) (Transformation|GetActorLocation)) Radius 12 "(R=0.000000,G=0.000000,B=0.000000,A=1.000000)" 0.0))